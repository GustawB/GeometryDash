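; BP_PlayerPawn is the player pawn Blueprint, which here only handles showing game menus based on flags in GDCGameInstance.
; BeginPlay caches the game instance and opens the main menu if its flag is set.
; Tick polls the level-completed flag, then the pause-menu flag.
; Each menu shown pauses the game, clears its flag, shows the mouse cursor and adds its widget to the viewport.
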(event `self.ReceiveBeginPlay`
  (bind _asgdcgame_instance (cast `GDCGameInstance` (`GameplayStatics.GetGameInstance`)))
  (bind _output_get (set `self.GDCGame Instance Reference` _asgdcgame_instance))
  (if (`GDCGameInstance.bCanShowMainMenu` _output_get)
    (`GameplayStatics.SetGamePaused` true)
    (bind _returnvalue (`|CreateWidget` "/Game/HUD/MainMenu_Widget.MainMenu_Widget_C"))
    (`UserWidget.AddToViewport` _returnvalue 0)
    (set `GDCGameInstance.bCanShowMainMenu` false (`self.GDCGame Instance Reference`))
    (set `PlayerController.bShowMouseCursor` true (`GameplayStatics.GetPlayerController` 0))))

(event `self.ReceiveTick`
  (params (DeltaSeconds :type "Float (single-precision)"))
  (if (`GDCGameInstance.bCanShowLevelCompleted` (`self.GDCGame Instance Reference`))
    (`GameplayStatics.SetGamePaused` true)
    (set `GDCGameInstance.bCanShowLevelCompleted` false (`self.GDCGame Instance Reference`))
    (set `PlayerController.bShowMouseCursor` true (`GameplayStatics.GetPlayerController` 0))
    (bind _returnvalue (`|CreateWidget` "/Game/HUD/LevelCompleted_Widget.LevelCompleted_Widget_C"))
    (`UserWidget.AddToViewport` _returnvalue 0)
    (elif (`GDCGameInstance.bCanShowPauseMenu` (`self.GDCGame Instance Reference`))
      (`GameplayStatics.SetGamePaused` true)
      (set `GDCGameInstance.bCanShowPauseMenu` false (`self.GDCGame Instance Reference`))
      (set `PlayerController.bShowMouseCursor` true (`GameplayStatics.GetPlayerController` 0))
      (bind _returnvalue_2 (`|CreateWidget` "/Game/HUD/PauseMenu_WIdget.PauseMenu_WIdget_C"))
      (`UserWidget.AddToViewport` _returnvalue_2 0))))

(fn `UserConstructionScript`)